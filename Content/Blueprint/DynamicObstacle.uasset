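; DynamicObstacle is an obstacle actor that continuously spins and drifts through the world.
; BeginPlay picks a random rotator without roll as its RotationSpeed.
; Each Tick applies that local rotation and a world offset from Velocity, both scaled by delta time and swept for collision.
; Velocity is only read here, never assigned.
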(event `self.ReceiveBeginPlay`
  (set `self.RotationSpeed` (`KismetMathLibrary.RandomRotator` false)))

(event `self.ReceiveActorBeginOverlap`
  (params (OtherActor :type "Actor Object Reference")))

(event `self.ReceiveTick`
  (params (DeltaSeconds :type "Float (single-precision)"))
  (`self.K2_AddActorLocalRotation` (* (`self.RotationSpeed`) DeltaSeconds) true)
  (`self.K2_AddActorWorldOffset` (* (`self.Velocity`) DeltaSeconds) true))

(fn `UserConstructionScript`
  (`parent.UserConstructionScript`))