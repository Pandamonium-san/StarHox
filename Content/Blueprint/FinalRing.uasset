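; FinalRing is the goal trigger in StarHox that ends the game in victory when the player pawn overlaps it.
; On overlap with StarHoxPawn_BP it shows the mouse cursor, pauses the game and sets the Victory flag on StarHoxGameMode_BP.
; It then creates the GameOverScreen widget and adds it to the viewport.
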(event `self.ReceiveBeginPlay`)

(event `self.ReceiveActorBeginOverlap`
  (params (OtherActor :type "Actor Object Reference"))
  (cast `/Game/Blueprint/StarHoxPawn_BP` OtherActor)
  (set `PlayerController.bShowMouseCursor` true (`GameplayStatics.GetPlayerController` 0))
  (`GameplayStatics.SetGamePaused` true)
  (bind _asstar_hox_game_mode_bp (cast `/Game/Blueprint/StarHoxGameMode_BP` (`GameplayStatics.GetGameMode`)))
  (set `StarHoxGameMode.bVictory` true _asstar_hox_game_mode_bp)
  (bind _returnvalue (`|CreateWidget` "/Game/Blueprint/GameOverScreen.GameOverScreen_C"))
  (`UserWidget.AddToViewport` _returnvalue 0))

(event `self.ReceiveTick`
  (params (DeltaSeconds :type "Float (single-precision)")))

(fn `UserConstructionScript`
  (`parent.UserConstructionScript`))