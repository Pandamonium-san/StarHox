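; StarHoxGameMode_BP is the game mode that triggers the game-over state when the player ship dies.
; Every tick it casts player pawn 0 to StarHoxPawn_BP and polls its CurrentHealth, printing a message if the cast fails.
; At zero health or below it shows the mouse cursor, adds a GameOverScreen widget to the viewport and pauses the game.
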(event `self.ReceiveBeginPlay`)

(event `self.ReceiveTick`
  (params (DeltaSeconds :type "Float (single-precision)"))
  (bind _asstar_hox_pawn_bp (cast `/Game/Blueprint/StarHoxPawn_BP` (`GameplayStatics.GetPlayerPawn` 0))
    (:`then`
      (if (>= 0.0 (`StarHoxPawn.CurrentHealth` _asstar_hox_pawn_bp))
        (set `PlayerController.bShowMouseCursor` true (`GameplayStatics.GetPlayerController` 0))
        (bind _returnvalue (`|CreateWidget` "/Game/Blueprint/GameOverScreen.GameOverScreen_C"))
        (`UserWidget.AddToViewport` _returnvalue 0)
        (`GameplayStatics.SetGamePaused` true)))
    (:`CastFailed`
      (`KismetSystemLibrary.PrintText` "Cast to pawn failed"))))

(fn `UserConstructionScript`)